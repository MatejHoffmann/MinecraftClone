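; BP_MinecraftWorld is the world actor for a Minecraft-style game, handling player setup at start and render distance controls.
; On BeginPlay it shows the HUD crosshair and action bar and switches input to game only.
; It then constructs grass, dirt and stone BP_Block items and adds them to the first inventory slots of the player's character.
; Number keys 1 and 2 lower and raise the render distance.
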(event `self.ReceiveBeginPlay`
  (bind _returnvalue (`GameplayStatics.GetPlayerController` 0))
  (bind _asminecraft_hud (cast `MinecraftHUD` (`PlayerController.GetHUD` _returnvalue)))
  (`MinecraftHUD.ShowCrossHair` _asminecraft_hud)
  (`MinecraftHUD.ShowActionBar` _asminecraft_hud)
  (`WidgetBlueprintLibrary.SetInputMode_GameOnly` _returnvalue)
  (bind _asbp_minecraft_character (cast `/Game/World/BP_MinecraftCharacter` (`GameplayStatics.GetPlayerPawn` 0)))
  (bind _returnvalue_2 (`|GenericCreateObject` "/Game/Items/BP_Block.BP_Block_C"))
  (set `Item.Thumbnail` "/Game/Items/Images/grassblock.grassblock" _returnvalue_2)
  (set `BlockItem.Type` "GRASS" _returnvalue_2)
  (bind _inventorycomponent (`MinecraftCharacter.InventoryComponent` _asbp_minecraft_character))
  (`InventoryComponent.AddItem` _inventorycomponent _returnvalue_2 0)
  (bind _returnvalue_3 (`|GenericCreateObject` "/Game/Items/BP_Block.BP_Block_C"))
  (set `Item.Thumbnail` "/Game/Items/Images/DirtBlock.DirtBlock" _returnvalue_3)
  (set `BlockItem.Type` "DIRT" _returnvalue_3)
  (`InventoryComponent.AddItem` _inventorycomponent _returnvalue_3 1)
  (bind _returnvalue_4 (`|GenericCreateObject` "/Game/Items/BP_Block.BP_Block_C"))
  (set `Item.Thumbnail` "/Game/Items/Images/StoneBlock.StoneBlock" _returnvalue_4)
  (set `BlockItem.Type` "STONE" _returnvalue_4)
  (`InventoryComponent.AddItem` _inventorycomponent _returnvalue_4 2))

(event `Key|One`
  (params (Key :type "Key Structure"))
  (:`Pressed`
    (`self.RenderDistanceDown`)))

(event `Key|Two`
  (params (Key :type "Key Structure"))
  (:`Pressed`
    (`self.RenderDistanceUp`)))

(fn `UserConstructionScript`)