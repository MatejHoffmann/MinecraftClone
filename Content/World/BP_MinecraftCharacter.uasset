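; Blueprint for the Minecraft-style player character that smooths first-person camera height changes when crouching and standing.
; Crouch start and end store the current camera Z, stop the opposing timeline, and lerp toward the crouched or base eye height.
; Starting from the current height lets an interrupted transition reverse without snapping.
; An unconnected chain that would fill inventory slots with grass, dirt and stone blocks never runs.
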(event `self.ReceiveBeginPlay`
  (set `self.ZPosition` (`self.BaseEyeHeight`)))

(event `self.K2_OnEndCrouch`
  (params (HalfHeightAdjust :type "Float (single-precision)") (ScaledHalfHeightAdjust :type "Float (single-precision)"))
  (bind _firstpersoncameracomponent (`self.FirstPersonCameraComponent`))
  (bind (_relativelocation_x _relativelocation_y) (`KismetMathLibrary.BreakVector` (`SceneComponent.RelativeLocation` _firstpersoncameracomponent)))
  (bind (_relativelocation_x_2 _relativelocation_y_2 _relativelocation_z) (`KismetMathLibrary.BreakVector` (`SceneComponent.RelativeLocation` (`self.FirstPersonCameraComponent`))))
  (set `self.ZPosition` _relativelocation_z)
  (`TimelineComponent.Stop` (`self.CrouchDown`))
  (bind (_direction _lerp_value) (`Timeline|CrouchUp` :!via `PlayFromStart`)
    (:`Update`
      (`SceneComponent.K2_SetRelativeLocation` _firstpersoncameracomponent (`KismetMathLibrary.MakeVector` _relativelocation_x _relativelocation_y (`KismetMathLibrary.Lerp` (`self.ZPosition`) (`self.BaseEyeHeight`) _lerp_value)) false false))))

(event `self.K2_OnStartCrouch`
  (params (HalfHeightAdjust :type "Float (single-precision)") (ScaledHalfHeightAdjust :type "Float (single-precision)"))
  (bind _firstpersoncameracomponent (`self.FirstPersonCameraComponent`))
  (bind (_relativelocation_x _relativelocation_y) (`KismetMathLibrary.BreakVector` (`SceneComponent.RelativeLocation` _firstpersoncameracomponent)))
  (bind (_relativelocation_x_2 _relativelocation_y_2 _relativelocation_z) (`KismetMathLibrary.BreakVector` (`SceneComponent.RelativeLocation` (`self.FirstPersonCameraComponent`))))
  (set `self.ZPosition` _relativelocation_z)
  (`TimelineComponent.Stop` (`self.CrouchUp`))
  (bind (_direction _lerp_value) (`Timeline|CrouchDown` :!via `PlayFromStart`)
    (:`Update`
      (`SceneComponent.K2_SetRelativeLocation` _firstpersoncameracomponent (`KismetMathLibrary.MakeVector` _relativelocation_x _relativelocation_y (`KismetMathLibrary.Lerp` (`self.ZPosition`) (`self.CrouchedEyeHeight`) _lerp_value)) false false))))

(fn `UserConstructionScript`)